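; Player character for RLGame that collects objective cubes, ends the level and provides camera panning.
; On Hit, it destroys an objective cube and increments the HUD component's score, or destroys a level-end actor and prints a win message.
; Helper functions step the camera in world X and Y by CameraMovementSpeed or snap it to a fixed center position.
; The level-end branch has no score check or level load, despite its comment.
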(event `self.ReceiveHit`
  (params (MyComp :type "PrimitiveComponent Object Reference") (Other :type "Actor Object Reference") (OtherComp :type "PrimitiveComponent Object Reference") (bSelfMoved :type Boolean) (HitLocation :type "Vector Structure") (HitNormal :type "Vector Structure") (NormalImpulse :type "Vector Structure") (Hit :type "HitResult Structure (by ref)"))
  ;[0 0.27 1] If objective hit, increment score
  (`/Engine/EditorBlueprintResources/StandardMacros.IsValid` Other
    (:`Is Valid`
      (bind _asbp_objective_cube (cast `/Game/RLGame/Objects/Actors/BP_ObjectiveCube` Other)
        (:`then`
          (`self.K2_DestroyActor` _asbp_objective_cube)
          (`GameplayStatics.GetActorOfClass` "/Game/RLGame/Objects/Actors/BP_LevelEnd.BP_LevelEnd_C")
          (`/Game/RLGame/Core/Player/Components/BP_Score_Component.IncrementScore` (`self.BP_Hud_Component`)))
        (:`CastFailed`
          ;[0 0.2689 1] When level end hit and game has ended, load next level
          (bind _asbp_level_end (cast `/Game/RLGame/Objects/Actors/BP_LevelEnd` Other))
          (`self.K2_DestroyActor` _asbp_level_end)
          (`KismetSystemLibrary.PrintString` "YOU WIN"))))))

(fn `CenterCamera`
  (`SceneComponent.K2_SetWorldLocation` (`self.Camera`) (200.0 1800.0 1000.0) false false))

(fn `MoveCameraDown`
  (bind (_returnvalue_x _returnvalue_y _returnvalue_z) (`KismetMathLibrary.BreakVector` (`SceneComponent.K2_GetComponentLocation` (`self.Camera`))))
  (`SceneComponent.K2_SetWorldLocation` (`self.Camera`) (`KismetMathLibrary.MakeVector` (- _returnvalue_x (`self.CameraMovementSpeed`)) _returnvalue_y _returnvalue_z) false false))

(fn `MoveCameraLeft`
  (bind (_returnvalue_x _returnvalue_y _returnvalue_z) (`KismetMathLibrary.BreakVector` (`SceneComponent.K2_GetComponentLocation` (`self.Camera`))))
  (`SceneComponent.K2_SetWorldLocation` (`self.Camera`) (`KismetMathLibrary.MakeVector` _returnvalue_x (- _returnvalue_y (`self.CameraMovementSpeed`)) _returnvalue_z) false false))

(fn `MoveCameraRight`
  (bind (_returnvalue_x _returnvalue_y _returnvalue_z) (`KismetMathLibrary.BreakVector` (`SceneComponent.K2_GetComponentLocation` (`self.Camera`))))
  (`SceneComponent.K2_SetWorldLocation` (`self.Camera`) (`KismetMathLibrary.MakeVector` _returnvalue_x (+ _returnvalue_y (`self.CameraMovementSpeed`)) _returnvalue_z) false false))

(fn `MoveCameraUp`
  (bind (_returnvalue_x _returnvalue_y _returnvalue_z) (`KismetMathLibrary.BreakVector` (`SceneComponent.K2_GetComponentLocation` (`self.Camera`))))
  (`SceneComponent.K2_SetWorldLocation` (`self.Camera`) (`KismetMathLibrary.MakeVector` (+ _returnvalue_x (`self.CameraMovementSpeed`)) _returnvalue_y _returnvalue_z) false false))

(fn `UserConstructionScript`)