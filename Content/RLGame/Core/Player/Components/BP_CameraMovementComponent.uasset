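; BP_CameraMovementComponent is a player component that turns directional input into camera movement on the RL player character.
; It handles the left, right, up and down Enhanced Input actions, each fetching the RL player character and calling its matching MoveCamera function.
; The component holds no movement logic itself; the character performs the actual camera motion.
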(event `EnhancedInput|/Game/RLGame/Input/IA_MoveLeft`
  (params (ActionValue :type Boolean) (ElapsedSeconds :type "Float (double-precision)") (TriggeredSeconds :type "Float (double-precision)") (InputAction :type "InputAction Object Reference" :default "/Game/RLGame/Input/IA_MoveLeft.IA_MoveLeft"))
  (:`Triggered`
    (`/Game/RLGame/Core/Player/BP_Character.MoveCameraLeft` (`/Game/RLGame/Core/BPFL_Core.GetRLPlayerCharacter`))))

(event `EnhancedInput|/Game/RLGame/Input/IA_MoveRight`
  (params (ActionValue :type Boolean) (ElapsedSeconds :type "Float (double-precision)") (TriggeredSeconds :type "Float (double-precision)") (InputAction :type "InputAction Object Reference" :default "/Game/RLGame/Input/IA_MoveRight.IA_MoveRight"))
  (:`Triggered`
    (`/Game/RLGame/Core/Player/BP_Character.MoveCameraRight` (`/Game/RLGame/Core/BPFL_Core.GetRLPlayerCharacter`))))

(event `EnhancedInput|/Game/RLGame/Input/IA_MoveUp`
  (params (ActionValue :type Boolean) (ElapsedSeconds :type "Float (double-precision)") (TriggeredSeconds :type "Float (double-precision)") (InputAction :type "InputAction Object Reference" :default "/Game/RLGame/Input/IA_MoveUp.IA_MoveUp"))
  (:`Triggered`
    (`/Game/RLGame/Core/Player/BP_Character.MoveCameraUp` (`/Game/RLGame/Core/BPFL_Core.GetRLPlayerCharacter`))))

(event `EnhancedInput|/Game/RLGame/Input/IA_MoveDown`
  (params (ActionValue :type Boolean) (ElapsedSeconds :type "Float (double-precision)") (TriggeredSeconds :type "Float (double-precision)") (InputAction :type "InputAction Object Reference" :default "/Game/RLGame/Input/IA_MoveDown.IA_MoveDown"))
  (:`Triggered`
    (`/Game/RLGame/Core/Player/BP_Character.MoveCameraDown` (`/Game/RLGame/Core/BPFL_Core.GetRLPlayerCharacter`))))