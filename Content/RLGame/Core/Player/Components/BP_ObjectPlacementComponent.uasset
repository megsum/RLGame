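; Player component for placing objects on a ground grid with the mouse, using Enhanced Input.
; A cursor trace accepts hits below GroundHeight and snaps them to a 100-unit grid at fixed height.
; A preview actor follows that point each tick, and confirming spawns the ObjectData actor class there.
; Cancel ends placement or, when idle, attempts to destroy an off-ground hit actor, though that trace branch returns no HitActor.
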(event `self.ReceiveTick`
  (params (DeltaSeconds :type "Float (single-precision)"))
  (`parent.ReceiveTick` DeltaSeconds)
  (`self.UpdatePreviewActorLocation`))

(event `self.ReceiveBeginPlay`
  (`parent.ReceiveBeginPlay`)
  (`self.SpawnPreviewActor`)
  (`self.HidePreviewActor`))

(event `EnhancedInput|/Game/RLGame/Input/IA_PlaceObject`
  (params (ActionValue :type Boolean) (ElapsedSeconds :type "Float (double-precision)") (TriggeredSeconds :type "Float (double-precision)") (InputAction :type "InputAction Object Reference" :default "/Game/RLGame/Input/IA_PlaceObject.IA_PlaceObject"))
  (:`Completed`
    (`self.ConfirmObjectPlacement`)))

(event `EnhancedInput|/Game/RLGame/Input/IA_Cancel`
  (params (ActionValue :type Boolean) (ElapsedSeconds :type "Float (double-precision)") (TriggeredSeconds :type "Float (double-precision)") (InputAction :type "InputAction Object Reference" :default "/Game/RLGame/Input/IA_Cancel.IA_Cancel"))
  (bind (_returnvalue _isonground _hitactor) (`self.GetMouseLocationOnGrid`))
  (:`Completed`
    (if (`self.bIsPlacementActive`)
      (`self.StopPlacingObject`)
      (`self.HidePreviewActor`)
      (elif (not _isonground)
        (`/Engine/EditorBlueprintResources/StandardMacros.IsValid` _hitactor
          (:`Is Valid`
            (`Actor.K2_DestroyActor` _hitactor)))))))

(fn `ConfirmObjectPlacement`
  (bind (_returnvalue _isonground) (`self.GetMouseLocationOnGrid`))
  (bind (_object_data_name _object_data_texture _object_data_actor) (break `/Game/RLGame/Objects/S_ObjectDefinition` (`self.Object Data`)))
  (bind (_object_data_name_2 _object_data_texture_2 _object_data_actor_2) (break `/Game/RLGame/Objects/S_ObjectDefinition` (`self.Object Data`)))
  (if (`KismetSystemLibrary.IsValidClass` _object_data_actor_2)
    (if _isonground
      (`|SpawnActorFromClass` _object_data_actor (`KismetMathLibrary.MakeTransform` _returnvalue) "Undefined" "MultiplyWithRoot" null null))))

(fn `GetMouseLocationOnGrid`
  (returns (ReturnValue :type "Vector Structure") (IsOnGround :type Boolean) (HitActor :type "Actor Object Reference"))
  (locals (GroundHeight :type "Float (double-precision)" :default -99.5))
  (bind (_worldlocation _worlddirection) (`PlayerController.DeprojectMousePositionToWorld` (`/Game/RLGame/Core/BPFL_Core.GetRLPlayerController`)))
  (bind _outhit (`KismetSystemLibrary.LineTraceSingle` _worldlocation (+ _worldlocation (* _worlddirection 5000.0)) "TraceTypeQuery1"))
  (bind (_bblockinghit _binitialoverlap _time _distance _location _impactpoint _normal _impactnormal _physmat _hitactor) (`GameplayStatics.BreakHitResult` _outhit))
  (if (< (.z _location) (`local.GroundHeight`))
    (return (`KismetMathLibrary.MakeVector` (`KismetMathLibrary.Conv_IntToDouble` (* (`KismetMathLibrary.Round` (/ (.x _location) 100.0)) 100)) (`KismetMathLibrary.Conv_IntToDouble` (* (`KismetMathLibrary.Round` (/ (.y _location) 100.0)) 100)) -50.0) true _hitactor)
    (else
      (return (0.0 0.0 0.0) false null))))

(fn `HidePreviewActor`
  (`Actor.SetActorHiddenInGame` (`self.PreviewActor`) true))

(fn `ShowPreviewActor`
  (`Actor.SetActorHiddenInGame` (`self.PreviewActor`) false))

(fn `SpawnPreviewActor`
  (bind _returnvalue (`|SpawnActorFromClass` "/Game/RLGame/Objects/Actors/BP_PreviewActor.BP_PreviewActor_C" (`KismetMathLibrary.MakeTransform` (0.0 0.0 0.0)) "Undefined" "MultiplyWithRoot" null null))
  (set `self.PreviewActor` _returnvalue))

(fn `StartPlacingObject`
  (params (ObjectData :type "/Game/RLGame/Objects/S_ObjectDefinition Structure"))
  (set `self.Object Data` ObjectData)
  (`self.ShowPreviewActor`)
  (set `self.bIsPlacementActive` true))

(fn `StopPlacingObject`
  (set `self.Object Data` (struct))
  (`self.HidePreviewActor`)
  (set `self.bIsPlacementActive` false))

(fn `UpdatePreviewActorLocation`
  (bind _previewactor (`self.PreviewActor`)
    (:`then`
      (`Actor.K2_SetActorLocation` _previewactor (`self.GetMouseLocationOnGrid`) false false))
    (:`else`)))