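; Player controller for the RL game that switches between edit and simulation modes, starting in edit mode.
; Each mode change adds or removes the edit input mapping context and adds that mode's widget to the viewport.
; While simulating, Tick steers the pawn as the RL agent straight toward GridWorldVisualizer's current location using movement input.
; Object placement only prints, and the click-to-move helpers are not called here.
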(event `self.ReceiveBeginPlay`
  (`parent.ReceiveBeginPlay`)
  (`self.Initialize`))

(event `EnhancedInput|/Game/RLGame/Input/IA_PlaceObject`
  (params (ActionValue :type Boolean) (ElapsedSeconds :type "Float (double-precision)") (TriggeredSeconds :type "Float (double-precision)") (InputAction :type "InputAction Object Reference" :default "/Game/RLGame/Input/IA_PlaceObject.IA_PlaceObject"))
  (:`Completed`
    (`KismetSystemLibrary.PrintString` "Place Object")))

(event `self.ReceiveTick`
  (params (DeltaSeconds :type "Float (single-precision)"))
  (bind (_hit _location) (`self.GetLocation`))
  ;[1 1 1] Move RL Agent to location on tick
  (`parent.ReceiveTick` DeltaSeconds)
  (if (`self.bIsSimulationRunning`)
    (if _hit
      (bind _output_get (set `self.CachedDestination` _location))
      (`self.Follow` _output_get))))

(fn `Follow`
  (params (Location :type "Vector Structure"))
  (bind _returnvalue (`self.K2_GetPawn`))
  (`Pawn.AddMovementInput` _returnvalue (`KismetMathLibrary.GetDirectionUnitVector` (`self.K2_GetActorLocation` _returnvalue) Location) 1.0 false))

(fn `GetLocation`
  (returns (Hit :type Boolean) (Location :type "Vector Structure"))
  ;[1 1 1] Get the latest location from the GridWorldVisualizer
  (return true (`GridWorldVisualizer.CurrentLocation` (`self.GridWorldVisualizer`))))

(fn `GetLocationUnderCursor`
  (returns (Hit :type Boolean) (Location :type "Vector Structure"))
  (bind (_bblockinghit _binitialoverlap _time _distance _location) (`GameplayStatics.BreakHitResult` (`self.GetHitResultUnderCursorByChannel` "TraceTypeQuery1")))
  (return _bblockinghit _location))

(fn `Initialize`
  (`self.StopSimulation`))

(fn `MoveTo`
  (params (Location :type "Vector Structure"))
  (`AIBlueprintHelperLibrary.SimpleMoveToLocation` self Location)
  (`NiagaraFunctionLibrary.SpawnSystemAtLocation` (`self.FXCursor`) Location))

(fn `StartSimulation`
  (set `self.bIsSimulationRunning` true)
  (`EnhancedInputSubsystemInterface.RemoveMappingContext` (subsystem `EnhancedInputLocalPlayerSubsystem`) "/Game/RLGame/Input/IMC_EditMode.IMC_EditMode" (struct))
  (bind _returnvalue (`|CreateWidget` "/Game/RLGame/UI/WBP_PlayMode.WBP_PlayMode_C"))
  (`UserWidget.AddToViewport` _returnvalue 0))

(fn `StopSimulation`
  (bind _returnvalue (subsystem `EnhancedInputLocalPlayerSubsystem`))
  (bind _returnvalue_2 (`|CreateWidget` "/Game/RLGame/UI/WBP_EditMode.WBP_EditMode_C"))
  (`UserWidget.AddToViewport` _returnvalue_2 0)
  (`/Engine/EditorBlueprintResources/StandardMacros.IsValid` _returnvalue
    (:`Is Valid`
      (`EnhancedInputSubsystemInterface.AddMappingContext` _returnvalue "/Game/RLGame/Input/IMC_EditMode.IMC_EditMode" 0 (struct))
      (set `self.bIsSimulationRunning` false))))

(fn `UserConstructionScript`)