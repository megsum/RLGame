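; Player character Blueprint that handles objective pickup and level completion through its Hit event.
; Hitting a BP_ObjectiveCube destroys it, then passes the WinningScore from the level's BP_LevelEnd actor to the HUD component's IncrementScore.
; Hitting BP_LevelEnd once its GameEnded flag is set only prints a win message; no next-level load is implemented here.
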(event `self.ReceiveHit`
  (params (MyComp :type "PrimitiveComponent Object Reference") (Other :type "Actor Object Reference") (OtherComp :type "PrimitiveComponent Object Reference") (bSelfMoved :type Boolean) (HitLocation :type "Vector Structure") (HitNormal :type "Vector Structure") (NormalImpulse :type "Vector Structure") (Hit :type "HitResult Structure (by ref)"))
  ;[0 0.27 1] If objective hit, increment score
  (`/Engine/EditorBlueprintResources/StandardMacros.IsValid` Other
    (:`Is Valid`
      (bind _asbp_objective_cube (cast `/Game/TopDown/Blueprints/BP_ObjectiveCube` Other)
        (:`then`
          (`self.K2_DestroyActor` _asbp_objective_cube)
          (bind _returnvalue (`GameplayStatics.GetActorOfClass` "/Game/TopDown/Blueprints/BP_LevelEnd.BP_LevelEnd_C"))
          (`/Game/RLGame/UI/BP_Hud_Component.IncrementScore` (`self.BP_Hud_Component`) (`/Game/TopDown/Blueprints/BP_LevelEnd.WinningScore` _returnvalue)))
        (:`CastFailed`
          ;[0 0.2689 1] When level end hit and game has ended, load next level
          (bind _asbp_level_end (cast `/Game/TopDown/Blueprints/BP_LevelEnd` Other))
          (if (`/Game/TopDown/Blueprints/BP_LevelEnd.Game Ended` _asbp_level_end)
            (`KismetSystemLibrary.PrintString` "YOU WIN")))))))

(fn `UserConstructionScript`)