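; Game mode for RLGame that builds an integer grid representation of the level and binds to the RL player controller's simulation-started event on BeginPlay.
; GenerateGridWorld fires debug-drawn downward line traces across grid cells, mapping each hit actor's first gameplay tag to a GridWorldObjects data table row.
; Found values are appended to GridWorld.
; The inner loop starts at the outer index, so only a triangular half of the grid is sampled.
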(event `self.ReceiveBeginPlay`
  (add `/Game/RLGame/Core/BP_PlayerController.OnSimulationStarted` (`/Game/RLGame/Core/BPFL_Core.GetRLPlayerController`) (`|CreateDelegate` :!event `GenerateGridWorld`)))

(fn `GenerateGridWorld`
  (for _index (range 11)
    (for _index_2 (range _index 11)
      (bind _returnvalue (* (`KismetMathLibrary.Conv_IntToDouble` _index) 100.0))
      (bind _returnvalue_2 (* (`KismetMathLibrary.Conv_IntToDouble` _index_2) 100.0))
      (bind _outhit (`KismetSystemLibrary.LineTraceSingleForObjects` :`Start` (`KismetMathLibrary.MakeVector` _returnvalue _returnvalue_2) :`End` (`KismetMathLibrary.MakeVector` (+ _returnvalue 50.0) (+ _returnvalue_2 50.0) -100.0) :`ObjectTypes` (`self.E_ObjectTypes`) :`DrawDebugType` "ForDuration"))
      (bind _tagcontainer (message `GameplayTagAssetInterface.GetOwnedGameplayTags` (`.HitActor` (`GameplayStatics.BreakHitResult` _outhit))))
      (bind _returnvalue_3 (`|GetDataTableRow` "/Game/RLGame/GridWorld/GridWorldObjects.GridWorldObjects" (`BlueprintGameplayTagLibrary.GetTagName` (`|GetArrayItem` (`BlueprintGameplayTagLibrary.BreakGameplayTagContainer` _tagcontainer))))
        (:`then`
          (`KismetArrayLibrary.Array_Add` (`self.GridWorld`) (`.IntValue_6_214C4A3F4B923EC1F916789CDE4A5741` (break `/Game/RLGame/GridWorld/S_ObjectToInt` _returnvalue_3)))
          (`KismetSystemLibrary.PrintText` "Hello"))))))

(fn `UserConstructionScript`)