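; Game mode for a reinforcement-learning game that converts placed level objects into an integer GridWorld array.
; BeginPlay binds a handler to the RL player controller's simulation-started event.
; GenerateGridWorld line-traces at 100-unit steps, matching each hit BP_Object's gameplay tag to a GridWorldObjects table value, with misses scored as negative reward.
; The inner loop starts at the outer index, so only a triangular half of the grid is sampled.
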(event `self.ReceiveBeginPlay`
  (add `/Game/RLGame/Core/BP_PlayerController.OnSimulationStarted` (`/Game/RLGame/Core/BPFL_Core.GetRLPlayerController`) (`|CreateDelegate` :!event `GenerateGridWorld`)))

(fn `GenerateGridWorld`
  (locals (GameplayTagInt :type Integer))
  (for _index (range 51)
    (for _index_2 (range _index 51)
      (bind _returnvalue (* (`KismetMathLibrary.Conv_IntToDouble` _index) 100.0))
      (bind _returnvalue_2 (* (`KismetMathLibrary.Conv_IntToDouble` _index_2) 100.0))
      (bind _outhit (`KismetSystemLibrary.LineTraceSingleForObjects` (`KismetMathLibrary.MakeVector` _returnvalue _returnvalue_2 100.0) (`KismetMathLibrary.MakeVector` (+ _returnvalue 50.0) (+ _returnvalue_2 50.0) -100.0) (`self.E_ObjectTypes`)))
      (bind _asbp_object (cast `/Game/RLGame/Objects/Actors/BP_Object` (`.HitActor` (`GameplayStatics.BreakHitResult` _outhit)))
        (:`then`
          (bind _outrownames (`DataTableFunctionLibrary.GetDataTableRowNames` "/Game/RLGame/GridWorld/GridWorldObjects.GridWorldObjects"))
          (for _array_element _outrownames
            (bind _returnvalue_3 (`|GetDataTableRow` "/Game/RLGame/GridWorld/GridWorldObjects.GridWorldObjects" _array_element)
              (:`then`
                (if (== (`/Game/RLGame/Objects/Actors/BP_Object.GameplayTag` _asbp_object) (break `/Game/RLGame/GridWorld/S_ObjectToInt` _returnvalue_3))
                  (set `local.GameplayTagInt` (`.IntValue_6_214C4A3F4B923EC1F916789CDE4A5741` (break `/Game/RLGame/GridWorld/S_ObjectToInt` _returnvalue_3)))
                  (break)))))
          (bind _returnvalue_4 (`KismetArrayLibrary.Array_Add` (`self.GridWorld`) (`local.GameplayTagInt`)))
          (`KismetSystemLibrary.PrintString` (`KismetStringLibrary.Conv_IntToString` _returnvalue_4)))
        (:`CastFailed`
          ;[1 1 1] If we don't hit anything, make that area negative rreward
          (`KismetArrayLibrary.Array_Add` (`self.GridWorld`) -100))))))

(fn `UserConstructionScript`)